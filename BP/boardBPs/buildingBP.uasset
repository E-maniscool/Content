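; A building actor for a board, which shows open placement options around itself and can be highlighted.
; The placement glow event shows each of four Glow components only if nothing overlaps it, or hides all four.
; The red glow event toggles custom depth rendering on the Cube for highlighting.
; The first actor overlap, gated by DoOnce, sets OverlappingHeald on every TopDownPawnBP in the level.
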(event Custom|place%20option%20glow
  (params (should%20glow :type Boolean))
  (bind _glow1 (Variables|Default|Getglow1))
  (bind _glow2 (Variables|Default|Getglow2))
  (bind _glow1_2 (Variables|Default|Getglow1))
  (bind _glow3 (Variables|Default|Getglow3))
  (bind _glow4 (Variables|Default|Getglow4))
  (if should%20glow
    (Utilities|IsValid (Utilities|Array|Get(acopy) (Collision|GetOverlappingActors _glow1 0 :!class /Script/Engine.PrimitiveComponent))
      (:Is%20Valid
        (Rendering|SetVisibility _glow1_2 false false))
      (:Is%20Not%20Valid
        (Rendering|SetVisibility _glow1_2 true false)))
    (Utilities|IsValid (Utilities|Array|Get(acopy) (Collision|GetOverlappingActors _glow2 0 :!class /Script/Engine.PrimitiveComponent))
      (:Is%20Valid
        (Rendering|SetVisibility _glow2 false false))
      (:Is%20Not%20Valid
        (Rendering|SetVisibility _glow2 true false)))
    (Utilities|IsValid (Utilities|Array|Get(acopy) (Collision|GetOverlappingActors _glow3 0 :!class /Script/Engine.PrimitiveComponent))
      (:Is%20Valid
        (Rendering|SetVisibility _glow3 false false))
      (:Is%20Not%20Valid
        (Rendering|SetVisibility _glow3 true false)))
    (Utilities|IsValid (Utilities|Array|Get(acopy) (Collision|GetOverlappingActors _glow4 0 :!class /Script/Engine.PrimitiveComponent))
      (:Is%20Valid
        (Rendering|SetVisibility _glow4 false false))
      (:Is%20Not%20Valid
        (Rendering|SetVisibility _glow4 true false)))
    (else
      (Rendering|SetVisibility _glow1 false false))))

(event EventGlowRedBuddy
  (params (turn%20on :type Boolean))
  (Rendering|SetRenderCustomDepth (Variables|Default|GetCube) turn%20on))

(event Collision|EventActorBeginOverlap
  (params (OtherActor :type Actor%20Object%20Reference))
  (Utilities|FlowControl|DoOnce false
    (:Completed
      (bind _outactors (Actor|GetAllActorsOfClass "/Game/BP/topDownController/topDownPawnBP.topDownPawnBP_C"))
      (for _array_element _outactors
        (Variables|/Game/BP/topDownController/topDownPawnBP.topDownPawnBP_C|SetoverlappingHeald _array_element true)))))

(fn ConstructionScript)