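; Troop piece for a multiplayer board game, with selection highlights and meshes hidden from opponents.
; Selection shows any of four Glow markers with no overlapping actor and flags overlapping enemy troops and buildings through GlowRedBuddy, which toggles custom depth.
; The ownership check shows MeshRef to the owner, retrying until valid, and a plain cube to others.
; Placement plays a sound and shows the cube if Cloaked, otherwise MeshRef.
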(event Custom|all%20check%20if%20own
  (bind _mesh_ref (Variables|Default|Getmesh%20ref))
  (Collision|SetCollisionEnabled (Variables|Default|Getglow1) "NoCollision")
  (bind _astop_down_pawn_bp (Utilities|Casting|CastTotopDownPawnBP (Game|Player|GetPlayerPawn 0)))
  (if (== (Variables|/Game/BP/topDownController/topDownPawnBP.topDownPawnBP_C|Getmy%20index _astop_down_pawn_bp) (Variables|Default|Getowner%20index))
    (Utilities|IsValid _mesh_ref :!label _label
      (:Is%20Valid
        (Development|PrintString (Utilities|GetDisplayName _mesh_ref) true true "(R=0.091038,G=1.000000,B=0.000000,A=1.000000)")
        (Components|StaticMesh|SetStaticMesh (Variables|Default|GetCube) _mesh_ref))
      (:Is%20Not%20Valid
        (Utilities|FlowControl|Delay 0.1)
        (goto _label)))
    (else
      (Components|StaticMesh|SetStaticMesh (Variables|Default|GetCube) "/Engine/BasicShapes/Cube.Cube"))))

(event Custom|is%20placed%20multi
  (Variables|Default|Setis%20placed true)
  (Audio|PlaySound2D "/Game/SFX/tap_Cue.tap_Cue" 1.0 1.0 0.0 0 0)
  (if (Variables|Default|Getis%20placed)
    (if (Variables|Default|Getcloaked)
      (bind _astop_down_pawn_bp (Utilities|Casting|CastTotopDownPawnBP (Game|Player|GetPlayerPawn 0)))
      (Components|StaticMesh|SetStaticMesh (Variables|Default|GetCube) "/Engine/BasicShapes/Cube.Cube")
      (else
        (Components|StaticMesh|SetStaticMesh (Variables|Default|GetCube) (Variables|Default|Getmesh%20ref))))))

(event Custom|is%20placed%20server
  (CallFunction|IsPlacedMulti))

(event Custom|im%20selected
  (params (select :type Boolean))
  (bind _red_guys (Variables|Default|Getred%20guys))
  (bind _glow2 (Variables|Default|Getglow2))
  (bind _glow1 (Variables|Default|Getglow1))
  (bind _glow3 (Variables|Default|Getglow3))
  (bind _glow4 (Variables|Default|Getglow4))
  (bind _glow1_2 (Variables|Default|Getglow1))
  (Variables|Default|SetSelected select)
  (if select
    (Collision|SetCollisionEnabled _glow1_2 "QueryAndPhysics")
    (for _array_element (Collision|GetOverlappingActors "troopBP_C" :!class /Script/Engine.Actor)
      (bind _astroop_bp (Utilities|Casting|CastTotroopBP _array_element))
      (if (not (== (Variables|troopBP_C|Getowner%20index _astroop_bp) (Variables|Default|Getowner%20index)))
        (Class|TroopsandBuildings|GlowRedBuddy(Message) _astroop_bp true)
        (Utilities|Array|Add (Variables|Default|Getred%20guys) _astroop_bp)))
    (for _array_element_2 (Collision|GetOverlappingActors "/Game/BP/boardBPs/buildingBP.buildingBP_C" :!class /Script/Engine.Actor)
      (bind _asbuilding_bp (Utilities|Casting|CastTobuildingBP _array_element_2))
      (if (not (== (Variables|/Game/BP/boardBPs/buildingBP.buildingBP_C|Getowner%20index _asbuilding_bp) (Variables|Default|Getowner%20index)))
        (Class|TroopsandBuildings|GlowRedBuddy(Message) _asbuilding_bp true)
        (Utilities|Array|Add (Variables|Default|Getred%20guys) _asbuilding_bp)))
    (Utilities|IsValid (Utilities|Array|Get(acopy) (Collision|GetOverlappingActors _glow1_2 0 :!class /Script/Engine.PrimitiveComponent))
      (:Is%20Valid
        (Rendering|SetVisibility _glow1 false false)
        (Collision|SetCollisionEnabled _glow1 "NoCollision"))
      (:Is%20Not%20Valid
        (Rendering|SetVisibility _glow1 true false)
        (Collision|SetCollisionEnabled _glow1 "QueryAndPhysics")))
    (Utilities|IsValid (Utilities|Array|Get(acopy) (Collision|GetOverlappingActors _glow2 0 :!class /Script/Engine.PrimitiveComponent))
      (:Is%20Valid
        (Rendering|SetVisibility _glow2 false false)
        (Collision|SetCollisionEnabled _glow2 "NoCollision"))
      (:Is%20Not%20Valid
        (Rendering|SetVisibility _glow2 true false)
        (Collision|SetCollisionEnabled _glow2 "QueryAndPhysics")))
    (Utilities|IsValid (Utilities|Array|Get(acopy) (Collision|GetOverlappingActors _glow3 0 :!class /Script/Engine.PrimitiveComponent))
      (:Is%20Valid
        (Rendering|SetVisibility _glow3 false false)
        (Collision|SetCollisionEnabled _glow3 "NoCollision"))
      (:Is%20Not%20Valid
        (Rendering|SetVisibility _glow3 true false)
        (Collision|SetCollisionEnabled _glow3 "QueryAndPhysics")))
    (Utilities|IsValid (Utilities|Array|Get(acopy) (Collision|GetOverlappingActors _glow4 0 :!class /Script/Engine.PrimitiveComponent))
      (:Is%20Valid
        (Rendering|SetVisibility _glow4 false false)
        (Collision|SetCollisionEnabled _glow4 "NoCollision"))
      (:Is%20Not%20Valid
        (Rendering|SetVisibility _glow4 true false)
        (Collision|SetCollisionEnabled _glow4 "QueryAndPhysics")))
    (else
      (Rendering|SetVisibility _glow1_2 false false)
      (Collision|SetCollisionEnabled _glow1_2 "NoCollision")
      (for _array_element_3 _red_guys
        (Class|TroopsandBuildings|GlowRedBuddy(Message) _array_element_3 false))
      (Utilities|Array|Clear _red_guys))))

(event Custom|server%20check%20all%20if%20own
  (CallFunction|AllCheckifOwn))

(event EventGlowRedBuddy
  (params (turn%20on :type Boolean))
  (Rendering|SetRenderCustomDepth (Variables|Default|GetCube) turn%20on))

(fn ConstructionScript)

(fn OnRepIsPlaced)

(fn OnRepCloaked)

(fn OnRepMeshRef)